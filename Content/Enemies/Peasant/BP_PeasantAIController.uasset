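; AI controller for the Peasant enemy that chases the player along a curved path and flags it to attack when close.
; Each tick outside an attack, it either sets CanAttack within a short range or calls MoveToPlayerInArc.
; That function interpolates yaw toward the player at a speed-scaled rate, then moves to a point just ahead, producing arcing turns.
; Failed or already-at-goal moves trigger an extra rotation interpolation.
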(event `self.ReceiveBeginPlay`
  (bind _asbp_peasant (cast `/Game/Enemies/Peasant/BP_Peasant` (`self.K2_GetPawn`)))
  (set `self.PeasantControlled` _asbp_peasant)
  (set `self.TargetPlayer` (`GameplayStatics.GetPlayerCharacter` 0)))

(event `self.ReceiveTick`
  (params (DeltaSeconds :type "Float (single-precision)"))
  (bind _peasantcontrolled (`self.PeasantControlled`))
  (bind _speed (`/Game/Enemies/Peasant/BP_Peasant.Speed` _peasantcontrolled))
  (bind _returnvalue (`MovementComponent.GetMaxSpeed` (`Character.CharacterMovement` _peasantcontrolled)))
  (if (`/Game/Enemies/Peasant/BP_Peasant.bIsAttacking` (`self.PeasantControlled`))
    _
    (elif (<= (`self.GetDistanceTo` (`self.TargetPlayer`) (`self.PeasantControlled`)) 100.0)
      (set `/Game/Enemies/Peasant/BP_Peasant.bCanAttack` true (`self.PeasantControlled`))
      (else
        (`self.MoveToPlayerInArc` (* (/ (`KismetMathLibrary.SelectFloat` _speed _returnvalue (> _speed 0.0)) _returnvalue) (`self.RotationToPlayerRate`)) DeltaSeconds)))))

(fn `MoveToPlayerInArc`
  (params (RotationSpeed :type "Float (double-precision)") (DeltaTime :type "Float (double-precision)"))
  (locals (TargetRotation :type "Rotator Structure" :default (struct)))
  (bind _peasantcontrolled (`self.PeasantControlled`))
  (bind (_returnvalue_x _returnvalue_y) (`KismetMathLibrary.BreakVector` (- (`self.K2_GetActorLocation` (`self.TargetPlayer`)) (`self.K2_GetActorLocation` (`self.PeasantControlled`)))))
  (bind _output_get (set `local.TargetRotation` (`KismetMathLibrary.RInterpTo` (`self.K2_GetActorRotation` (`self.PeasantControlled`)) (`KismetMathLibrary.Conv_VectorToRotator` (`KismetMathLibrary.MakeVector` _returnvalue_x _returnvalue_y)) (`local.DeltaTime`) (`local.RotationSpeed`))))
  (`self.K2_SetActorRotation` (`self.PeasantControlled`) _output_get false)
  (bind _returnvalue (`self.MoveToLocation` (+ (* (`self.GetActorForwardVector` _peasantcontrolled) 100) (`self.K2_GetActorLocation` _peasantcontrolled)) -1.0 true true false true null))
  (switch `EPathFollowingRequestResult` _returnvalue
    (:`Failed`
      _)
    (:`AlreadyAtGoal`
      _))
  (`self.K2_SetActorRotation` (`self.PeasantControlled`) (`KismetMathLibrary.RInterpTo` (`self.K2_GetActorRotation` (`self.PeasantControlled`)) (`local.TargetRotation`) (`local.DeltaTime`) 50.0) false))

(fn `UserConstructionScript`)