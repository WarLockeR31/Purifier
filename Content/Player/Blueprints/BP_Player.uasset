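; BP_Player is the player Blueprint, exposing health queries, healing and damage handling.
; GetCurrentHealth, GetMaxHealth, Heal and TakeDamage each forward directly to Health and return its result, so the player holds no health logic of its own.
; The event graph and construction script contain no logic.
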(event `self.ReceiveBeginPlay`)

(event `self.ReceiveTick`
  (params (DeltaSeconds :type "Float (single-precision)")))

(fn `GetCurrentHealth`
  (returns (ReturnValue :type "Float (single-precision)"))
  (return (`HealthComponent.GetCurrentHealth` (`self.Health`))))

(fn `GetMaxHealth`
  (returns (ReturnValue :type "Float (single-precision)"))
  (return (`HealthComponent.GetMaxHealth` (`self.Health`))))

(fn `Heal`
  (params (HealAmount :type "Float (single-precision)"))
  (returns (ReturnValue :type "Float (single-precision)"))
  (bind _returnvalue (`HealthComponent.Heal` (`self.Health`) HealAmount))
  (return _returnvalue))

(fn `TakeDamage`
  (params (DamageInfo :type "DamageInfo Structure (by ref)"))
  (returns (ReturnValue :type "Float (single-precision)"))
  (bind _returnvalue (`HealthComponent.TakeDamage` (`self.Health`) DamageInfo))
  (return _returnvalue))

(fn `UserConstructionScript`)